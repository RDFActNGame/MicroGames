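; BP_KEY is a pickup key that stays hidden and non-collidable until no BP_MovingTarget actors remain in the level.
; Tick polls all targets, using the index returned by an array Add as the count, and toggles visibility and collision.
; The first reveal plays a one-time explosion effect and sound.
; Player overlap then sets HasKey on BP_FirstPersonCharacter, plays a sound and destroys the key.
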(event OnComponentBeginOverlap(Collider)
  (params (OverlappedComponent :type Primitive%20Component%20Object%20Reference) (OtherActor :type Actor%20Object%20Reference) (OtherComp :type Primitive%20Component%20Object%20Reference) (OtherBodyIndex :type Integer) (bFromSweep :type Boolean) (SweepResult :type Hit%20Result%20Structure%20%28by%20ref%29))
  ;[0.02692 0.15 0 0.5] pick up + destroy key
  (if (and (== OtherActor (Variables|Default|GetAs%20BP%20First%20Person%20Character)) (Variables|Default|GetAllTargetsDestroyed))
    (Variables|/Game/FirstPerson/Blueprints/BP_FirstPersonCharacter.BP_FirstPersonCharacter_C|SetHasKey (Variables|Default|GetAs%20BP%20First%20Person%20Character) true)
    (Audio|PlaySoundatLocation "/Game/FPWeapon/Audio/FirstPersonTemplateWeaponFire02.FirstPersonTemplateWeaponFire02" (Transformation|GetActorLocation) "0, 0, 0" 1.0 1.0 0.0 0 0 0 0)
    (Actor|DestroyActor)))

(event EventBeginPlay
  ;[0.15 0.08644 0 0.5] Setup Key
  (bind _asbp_first_person_character (Utilities|Casting|CastToBP_FirstPersonCharacter (Game|GetPlayerCharacter 0)))
  (Variables|Default|SetAs%20BP%20First%20Person%20Character _asbp_first_person_character))

(event EventTick
  (params (DeltaSeconds :type Float%20%28single-precision%29))
  (bind _static_mesh_key (Variables|Default|GetStatic%20mesh_KEY))
  (bind _returnvalue (Transformation|GetWorldLocation _static_mesh_key))
  ;[0.15 0.15 0.15 0.5] Key-Visibility
  (bind _outactors (Actor|GetAllActorsOfClass "/Game/MicroGames/BP_MovingTarget.BP_MovingTarget_C"))
  (bind _returnvalue_2 (Utilities|Array|Add _outactors 0))
  (bind _output_get (Variables|Default|SetAllTargetsDestroyed (<= _returnvalue_2 0)))
  (Rendering|SetVisibility (Variables|Default|GetStatic%20mesh_KEY) _output_get true)
  (Collision|SetActorEnableCollision _output_get)
  ;[0.1189 0 0.8906 0.5] Key sound+effects
  (if (Variables|Default|GetAllTargetsDestroyed)
    (Utilities|FlowControl|DoOnce false
      (:Completed
        (Effects|SpawnEmitteratLocation "/Game/StarterContent/Particles/P_Explosion.P_Explosion" _returnvalue)
        (Audio|PlaySoundatLocation "/Game/StarterContent/Audio/Starter_Birds01.Starter_Birds01" _returnvalue "0, 0, 0" 1.0 1.0 0.0 0 0 0 0)))))

(fn ConstructionScript)