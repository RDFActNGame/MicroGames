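; Key-locked door for a micro game that swings open when the player enters its zone holding a key, with a status light.
; BeginPlay caches the first-person character and puts a dynamic emissive material on the door light.
; Overlap brightens the light, green with HasKey or red without; with the key, a Timeline lerps the door rotation 90 degrees.
; Leaving restores the dim warm light and reverses the Timeline to close the door.
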(event OnComponentBeginOverlap(DoorZone)
  (params (OverlappedComponent :type Primitive%20Component%20Object%20Reference) (OtherActor :type Actor%20Object%20Reference) (OtherComp :type Primitive%20Component%20Object%20Reference) (OtherBodyIndex :type Integer) (bFromSweep :type Boolean) (SweepResult :type Hit%20Result%20Structure%20%28by%20ref%29))
  ;[0 0.6087 1 0.5] light function
  (if (== OtherActor (Variables|Default|GetAs%20BP%20First%20Person%20Character))
    (Rendering|Material|SetScalarParameterValue (Variables|Default|Getdynamic%20material) "intensity" 1e+02 :!class /Script/Engine.MaterialInstanceDynamic)
    (if (Variables|/Game/FirstPerson/Blueprints/BP_FirstPersonCharacter.BP_FirstPersonCharacter_C|GetHasKey (Variables|Default|GetAs%20BP%20First%20Person%20Character))
      (Rendering|Material|SetVectorParameterValue (Variables|Default|Getdynamic%20material) "colour_param" "(R=0.066632,G=0.893750,B=0.000000,A=1.000000)" :!class /Script/Engine.MaterialInstanceDynamic)
      ;[0.007017 0.15 0 0.5] door open
      (bind _alpha (Timeline|Timeline Play)
        (:Update
          (Variables|Default|Setopening true)
          (Transformation|SetRelativeRotation (Variables|Default|GetSM_Door) (Math|Rotator|Lerp(Rotator) "0, 0, 0" "0.000000,90.000000,0.000000" _alpha) false false))
        (:Finished
          (Variables|Default|Setopening false)))
      (else
        (Rendering|Material|SetVectorParameterValue (Variables|Default|Getdynamic%20material) "colour_param" "(R=0.893750,G=0.001862,B=0.001862,A=1.000000)" :!class /Script/Engine.MaterialInstanceDynamic)))))

(event OnComponentEndOverlap(DoorZone)
  (params (OverlappedComponent :type Primitive%20Component%20Object%20Reference) (OtherActor :type Actor%20Object%20Reference) (OtherComp :type Primitive%20Component%20Object%20Reference) (OtherBodyIndex :type Integer))
  ;[1 1 1 0.5] light return
  (if (== OtherActor (Variables|Default|GetAs%20BP%20First%20Person%20Character))
    (Rendering|Material|SetScalarParameterValue (Variables|Default|Getdynamic%20material) "intensity" 1.0 :!class /Script/Engine.MaterialInstanceDynamic)
    (Rendering|Material|SetVectorParameterValue (Variables|Default|Getdynamic%20material) "colour_param" "(R=1.000000,G=0.917647,B=0.694118,A=1.000000)" :!class /Script/Engine.MaterialInstanceDynamic)
    ;[0.007017 0.15 0 0.5] door open
    (bind _alpha (Timeline|Timeline Reverse)
      (:Update
        (Variables|Default|Setopening true)
        (Transformation|SetRelativeRotation (Variables|Default|GetSM_Door) (Math|Rotator|Lerp(Rotator) "0, 0, 0" "0.000000,90.000000,0.000000" _alpha) false false))
      (:Finished
        (Variables|Default|Setopening false)))))

(event EventBeginPlay
  ;[0.3115 0.1508 0.07959 0.5] door set
  (bind _asbp_first_person_character (Utilities|Casting|CastToBP_FirstPersonCharacter (Game|GetPlayerCharacter 0)))
  (Variables|Default|SetAs%20BP%20First%20Person%20Character _asbp_first_person_character)
  (bind _returnvalue (Rendering|Material|CreateDynamicMaterialInstance "/Game/MicroGames/MI_emission.MI_emission" "None" "None" :!class /Script/Engine.KismetMaterialLibrary))
  (Variables|Default|Setdynamic%20material _returnvalue)
  (Rendering|Material|SetMaterial (Variables|Default|GetDoorLight) 0 (Variables|Default|Getdynamic%20material)))

(fn ConstructionScript)